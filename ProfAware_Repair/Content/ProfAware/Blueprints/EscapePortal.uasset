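; Level exit portal that switches on once the player has repaired every RepairStation, or shortly after start when AutoOn is set.
; It gathers the stations on BeginPlay and polls the player's repaired count on Tick, with a DoOnce guarding the delayed activation effect and sound.
; When the player overlaps the active portal, it plays a teleport sound, stops movement, fades to black and sets the character's Passed flag.
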(event OnComponentBeginOverlap(Box)
  (params (OverlappedComponent :type Primitive%20Component%20Object%20Reference) (OtherActor :type Actor%20Object%20Reference) (OtherComp :type Primitive%20Component%20Object%20Reference) (OtherBodyIndex :type Integer) (bFromSweep :type Boolean) (SweepResult :type Hit%20Result%20Structure%20%28by%20ref%29))
  (if (and (Variables|Default|GetOn) (== OtherActor (Game|GetPlayerCharacter 0)))
    (Audio|PlaySoundatLocation "/Game/ProfAware/Sound/teleport.teleport" (Transformation|GetActorLocation) "0, 0, 0" 1.0 1.0 0.0 0 0 0)
    (AI|Navigation|StopMovement (Game|GetPlayerController 0))
    (CameraFades|StartCameraFade :self (Game|GetPlayerCameraManager 0) :ToAlpha 1.0 :Duration 0.8 :bShouldFadeAudio true :bHoldWhenFinished true)
    (bind _asplayer_character_v2 (Utilities|Casting|CastToPlayerCharacterV2 (Game|GetPlayerCharacter 0)))
    (Variables|/Game/ProfAware/Blueprints/PlayerCharacterV2.PlayerCharacterV2_C|SetPassed _asplayer_character_v2 true)))

(event Custom|Turn%20Portal%20On
  (Components|Activation|Activate (Variables|Default|GetPortal%20Effect) false)
  (Audio|PlaySound2D "/Engine/VREditor/Sounds/UI/Dockable_Window_Pick_Up.Dockable_Window_Pick_Up" 1.0 1.0 0.0 0 0)
  (Variables|Default|SetOn true))

(event EventBeginPlay
  (Utilities|FlowControl|Delay 1.0)
  (bind _outactors (Actor|GetAllActorsOfClass "/Game/ProfAware/Blueprints/RepairStation.RepairStation_C"))
  (bind _output_get (Variables|Default|SetStations _outactors))
  (Actor|Tick|SetActorTickEnabled self true)
  (if (Variables|Default|GetAutoOn)
    (Utilities|FlowControl|Delay 3.0)
    (CallFunction|TurnPortalon)))

(event Collision|EventActorBeginOverlap
  (params (OtherActor :type Actor%20Object%20Reference)))

(event EventTick
  (params (DeltaSeconds :type Float%20%28single-precision%29))
  (bind _asplayer_character_v2 (Utilities|Casting|CastToPlayerCharacterV2 (Game|GetPlayerCharacter 0)))
  (if (== (Variables|/Game/ProfAware/Blueprints/PlayerCharacterV2.PlayerCharacterV2_C|GetTotalStationsRepaired _asplayer_character_v2) (Utilities|Array|Length (Variables|Default|GetStations)))
    (Utilities|FlowControl|DoOnce false
      (:Completed
        (Utilities|FlowControl|Delay 1.0)
        (CallFunction|TurnPortalon)))))

(fn ConstructionScript)