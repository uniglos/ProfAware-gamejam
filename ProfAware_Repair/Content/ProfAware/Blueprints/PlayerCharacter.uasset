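; Player character with directional movement, mouse-wheel camera zoom and an energy meter that quits the game when empty.
; A looping timer drains energy, while Tick refills it in recharge zones and applies GetRotation's results to body parts.
; Holding Shoot drives Delay-throttled line traces from Tick with random cone spread, damaging AI_Character.
; Shots add Niagara effects, sound, decals and debug-line tracers.
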(event Custom|Set%20Body%20Rotations
  (bind (_headrot _bodyrot _armsrot) (Utilities|GetRotation))
  (Transformation|SetWorldRotation (Variables|Character|GetMesh) _headrot false false)
  (Transformation|SetWorldRotation (Variables|Default|GetBody) _bodyrot false false)
  (Transformation|SetWorldRotation (Variables|Default|GetLeft%20Arm) _armsrot false false)
  (Transformation|SetWorldRotation (Variables|Default|GetRight%20Arm) _armsrot false false))

(event Custom|Consume%20Energy
  (Variables|Default|SetEnergy (- (Variables|Default|GetEnergy) 0.05)))

(event Custom|Recharging
  (if (and (Variables|Default|GetIn%20Recharge%20Zone) (Variables|Default|GetRechargeable?))
    (Utilities|FlowControl|Delay 0.5)
    (if (>= (Variables|Default|GetEnergy) 1.0)
      (Variables|Default|SetEnergy 1.0)
      (else
        (Variables|Default|SetEnergy (+ (Variables|Default|GetEnergy) 0.1))))))

(event Custom|Out%20Of%20Energy?
  (if (<= (Variables|Default|GetEnergy) 0.0)
    (Audio|PlaySound2D "/Engine/EditorSounds/Notifications/CompileFailed.CompileFailed" 1.0 1.0 0.0 0 0)
    (Game|QuitGame 0 "Quit" false)))

(event EventBeginPlay
  (Utilities|Time|SetTimerbyEvent (delegate Custom|Consume%20Energy) 2.0 true))

(event Collision|EventActorBeginOverlap
  (params (OtherActor :type Actor%20Object%20Reference)))

(event EventTick
  (params (DeltaSeconds :type Float%20%28single-precision%29))
  (bind _returnvalue (Transformation|GetActorLocation))
  (bind _barrel (Variables|Default|Getbarrel))
  (bind _barrel_2 (Variables|Default|Getbarrel))
  (bind _returnvalue_2 (Transformation|GetWorldLocation _barrel))
  (CallFunction|OutOfEnergy?)
  (CallFunction|Recharging)
  (CallFunction|SetBodyRotations)
  (if (Variables|Default|GetFiring)
    (Utilities|FlowControl|Delay 0.1)
    (Rendering|ToggleVisibility (Variables|Default|Getmuzzle%20light) false)
    (bind _outhit (Collision|LineTraceForObjects _returnvalue (+ _returnvalue (* (Math|Random|RandomUnitVectorinConeinDegrees (Math|Vector|GetForwardVector (Variables|Default|GetBody)) 1.0) 2e+03)) (Variables|Default|GetObject%20Types) false 0 "None"))
    (Niagara|SpawnSystematLocation "/Game/ProfAware/Effects/MuzzleFlashEffect.MuzzleFlashEffect" (Transformation|GetWorldLocation _barrel_2) (Math|Conversions|RotationFromXVector (* (Math|Vector|GetUpVector _barrel_2) -1.0)))
    (if (.bBlockingHit (Collision|BreakHitResult _outhit))
      (Rendering|Debug|DrawDebugLine _returnvalue_2 (.Location (Collision|BreakHitResult _outhit)) "(R=1.000000,G=1.000000,B=1.000000,A=1.000000)" 0.1 1.0)
      (else
        (Rendering|Debug|DrawDebugLine _returnvalue_2 (+ _returnvalue_2 (* (Math|Vector|GetUpVector _barrel) -2e+03)) "(R=1.000000,G=1.000000,B=1.000000,A=1.000000)" 0.1 1.0)))
    (Audio|PlaySoundatLocation "/Engine/VREditor/Sounds/UI/Laser_Push.Laser_Push" (.Location (Collision|BreakHitResult _outhit)) "0, 0, 0" 1.0 (Math|Random|RandomFloatinRange 1.0 1.5) 0.0 0 0 0)
    (Niagara|SpawnSystematLocation "/Game/ProfAware/Effects/ExplosionEffect.ExplosionEffect" (.Location (Collision|BreakHitResult _outhit)) (Math|Conversions|RotationFromXVector (.ImpactNormal (Collision|BreakHitResult _outhit))))
    (Rendering|Decal|SpawnDecalatLocation "/Game/ProfAware/Textures+Materials/oie_transparent_Mat.oie_transparent_Mat" "15.000000,3.000000,3.000000" (.ImpactPoint (Collision|BreakHitResult _outhit)) (Math|Conversions|RotationFromXVector (.ImpactNormal (Collision|BreakHitResult _outhit))) 4.0)
    (if (== (Utilities|GetClass (.HitActor (Collision|BreakHitResult _outhit))) "/Game/ProfAware/AI/AI_Character.AI_Character_C")
      (bind _asai_character (Utilities|Casting|CastToAI_Character (.HitActor (Collision|BreakHitResult _outhit))))
      (Default|TakeDamage _asai_character 3.0))))

(event Input|ActionEvents|InputActionShoot
  (params (Key :type Key%20Structure :default "None"))
  (:Pressed
    (Variables|Default|SetFiring true))
  (:Released
    (Variables|Default|SetFiring false)))

(event Input|AxisEvents|InputAxisLeft/Right
  (params (AxisValue :type Float%20%28single-precision%29))
  (Pawn|Input|AddMovementInput (Transformation|GetActorRightVector) AxisValue false))

(event Input|AxisEvents|InputAxisUp/Down
  (params (AxisValue :type Float%20%28single-precision%29))
  (Pawn|Input|AddMovementInput (Transformation|GetActorForwardVector) AxisValue false))

(event Input|MouseEvents|MouseWheelAxis
  (params (AxisValue :type Float%20%28single-precision%29))
  (bind _springarm (Variables|Default|GetSpringArm))
  (if (>= (Variables|/Script/Engine.SpringArmComponent|GetTargetArmLength _springarm) 1.2e+03)
    (Variables|/Script/Engine.SpringArmComponent|SetTargetArmLength _springarm 1199.0)
    (else
      (Variables|/Script/Engine.SpringArmComponent|SetTargetArmLength _springarm (- (Variables|/Script/Engine.SpringArmComponent|GetTargetArmLength _springarm) (* AxisValue 1e+02))))))

(fn ConstructionScript)