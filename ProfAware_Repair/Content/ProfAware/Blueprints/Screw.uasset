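; Screw is a short-lived effect actor that animates itself and then removes itself.
; On BeginPlay it plays its ActorSequence, waits five seconds and destroys the actor.
; Disconnected leftover logic would show the mouse cursor, move the actor to the point clicked under it and replay the sequence, but it never runs.
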(event EventBeginPlay
  (Sequencer|Player|Play (Variables|/Script/ActorSequence.ActorSequenceComponent|GetSequencePlayer (Variables|Default|GetActorSequence)) :!class /Script/MovieScene.MovieSceneSequencePlayer)
  (Utilities|FlowControl|Delay 5.0)
  (Actor|DestroyActor))

(event Collision|EventActorBeginOverlap
  (params (OtherActor :type Actor%20Object%20Reference)))

(event EventTick
  (params (DeltaSeconds :type Float%20%28single-precision%29)))

(fn ConstructionScript)