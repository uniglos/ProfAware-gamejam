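; Repairable lamp actor that acts as a player recharge zone once working.
; A broken lamp shows a red bulb and delayed Niagara effect until the player holds E inside FixArea.
; When working, it plays a one-shot shutter sound, turns white, and eases its light intensity and RechargeArea radius outward via per-tick Lerp.
; Overlap events and Tick set the player's fix and recharge flags.
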(event OnComponentBeginOverlap(FixArea)
  (params (OverlappedComponent :type Primitive%20Component%20Object%20Reference) (OtherActor :type Actor%20Object%20Reference) (OtherComp :type Primitive%20Component%20Object%20Reference) (OtherBodyIndex :type Integer) (bFromSweep :type Boolean) (SweepResult :type Hit%20Result%20Structure%20%28by%20ref%29))
  (if (Components|ComponentHasTag OtherComp "PlayerTorso")
    (Variables|Default|SetPlayerInRange true)
    (bind _asplayer_character (Utilities|Casting|CastToPlayerCharacter OtherActor))
    (Variables|/Game/ProfAware/Blueprints/PlayerCharacter.PlayerCharacter_C|SetInFixRange _asplayer_character true)))

(event OnComponentEndOverlap(FixArea)
  (params (OverlappedComponent :type Primitive%20Component%20Object%20Reference) (OtherActor :type Actor%20Object%20Reference) (OtherComp :type Primitive%20Component%20Object%20Reference) (OtherBodyIndex :type Integer))
  (if (Components|ComponentHasTag OtherComp "PlayerTorso")
    (Variables|Default|SetPlayerInRange false)
    (bind _asplayer_character (Utilities|Casting|CastToPlayerCharacter OtherActor))
    (Variables|/Game/ProfAware/Blueprints/PlayerCharacter.PlayerCharacter_C|SetInFixRange _asplayer_character false)))

(event OnComponentBeginOverlap(RechargeArea)
  (params (OverlappedComponent :type Primitive%20Component%20Object%20Reference) (OtherActor :type Actor%20Object%20Reference) (OtherComp :type Primitive%20Component%20Object%20Reference) (OtherBodyIndex :type Integer) (bFromSweep :type Boolean) (SweepResult :type Hit%20Result%20Structure%20%28by%20ref%29))
  (bind _returnvalue (Game|GetPlayerCharacter 0))
  (if (== OtherActor _returnvalue)
    (bind _asplayer_character (Utilities|Casting|CastToPlayerCharacter _returnvalue))
    (Variables|/Game/ProfAware/Blueprints/PlayerCharacter.PlayerCharacter_C|SetIn%20Recharge%20Zone _asplayer_character true)
    (Variables|Default|SetPlayerInRechargeRange true)))

(event OnComponentEndOverlap(RechargeArea)
  (params (OverlappedComponent :type Primitive%20Component%20Object%20Reference) (OtherActor :type Actor%20Object%20Reference) (OtherComp :type Primitive%20Component%20Object%20Reference) (OtherBodyIndex :type Integer))
  (bind _returnvalue (Game|GetPlayerCharacter 0))
  (if (== OtherActor _returnvalue)
    (bind _asplayer_character (Utilities|Casting|CastToPlayerCharacter _returnvalue))
    (Variables|/Game/ProfAware/Blueprints/PlayerCharacter.PlayerCharacter_C|SetIn%20Recharge%20Zone _asplayer_character false)
    (Variables|Default|SetPlayerInRechargeRange false)))

(event Custom|grow%20light
  (bind _recharge_area (Variables|Default|GetRecharge%20Area))
  (bind _lamp_area_light (Variables|Default|GetLamp%20Area%20Light))
  (if (not (Variables|Default|GetBroken?))
    (Components|Sphere|SetSphereRadius _recharge_area (Math|Float|Lerp (Variables|/Script/Engine.SphereComponent|GetSphereRadius _recharge_area) 8e+02 0.1) true)
    (Rendering|Components|Light|SetIntensity _lamp_area_light (Math|Float|Lerp (Variables|/Script/Engine.LightComponentBase|GetIntensity _lamp_area_light) 8e+03 0.1))))

(event EventBeginPlay
  (Variables|Default|SetPlayer (Game|GetPlayerCharacter 0)))

(event EventTick
  (params (DeltaSeconds :type Float%20%28single-precision%29))
  (bind _returnvalue (Game|GetPlayerCharacter 0))
  (CallFunction|GrowLight)
  (if (Variables|Default|GetBroken?)
    (if (Variables|Default|GetPlayerInRange)
      (if (> (Class|PlayerController|GetInputKeyTimeDown (Game|GetPlayerController 0) "E") 5.0)
        (Variables|Default|SetBroken? false))
      (else
        (Utilities|FlowControl|Delay 5.0)
        (Components|Activation|Activate (Variables|Default|GetNiagara) true)))
    (else
      (if (Variables|Default|GetPlayerInRechargeRange)
        (bind _asplayer_character (Utilities|Casting|CastToPlayerCharacter _returnvalue))
        (Variables|/Game/ProfAware/Blueprints/PlayerCharacter.PlayerCharacter_C|SetRechargeable? _asplayer_character true)
        (else
          (bind _asplayer_character_2 (Utilities|Casting|CastToPlayerCharacter _returnvalue))
          (Variables|/Game/ProfAware/Blueprints/PlayerCharacter.PlayerCharacter_C|SetRechargeable? _asplayer_character_2 false)))
      (Utilities|FlowControl|DoOnce false
        (:Completed
          (Audio|PlaySoundatLocation "/Engine/VREditor/Sounds/UI/Camera_Shutter.Camera_Shutter" (Transformation|GetActorLocation) "0, 0, 0" 1.0 1.0 0.0 0 0 0)
          (Rendering|Components|Light|SetLightColor (Variables|Default|GetLamp-Bulb%20Light) "(R=1.000000,G=1.000000,B=1.000000,A=1.000000)" true)
          (Rendering|SetVisibility (Variables|Default|GetLamp%20Area%20Light) true false))))))

(fn ConstructionScript
  (if (Variables|Default|GetBroken?)
    (Rendering|Components|Light|SetLightColor (Variables|Default|GetLamp-Bulb%20Light) "(R=1.000000,G=0.000000,B=0.000000,A=1.000000)" true)
    (Rendering|SetVisibility (Variables|Default|GetLamp%20Area%20Light) false false)))