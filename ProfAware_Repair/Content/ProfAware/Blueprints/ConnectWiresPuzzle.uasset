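; ConnectWiresPuzzle is an actor for a wire-connecting puzzle, so far only dragging a spline mesh wire with the mouse.
; BeginPlay shows the cursor, and while left mouse is held, Tick traces under it on Visibility.
; Each trace moves the mesh end to its start position plus the world impact point and draws a debug point there.
; Setting the start from the actor location is unwired, and no connection checks exist.
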(event EventBeginPlay
  (Variables|/Script/Engine.PlayerController|SetbShowMouseCursor (Game|GetPlayerController 0) true))

(event Collision|EventActorBeginOverlap
  (params (OtherActor :type Actor%20Object%20Reference)))

(event EventTick
  (params (DeltaSeconds :type Float%20%28single-precision%29))
  (bind _returnvalue (Game|GetPlayerController 0))
  (bind _splinemesh (Variables|Default|GetSplineMesh))
  (bind _hitresult (Game|Player|GetHitResultUnderCursorbyChannel _returnvalue "TraceTypeQuery1" true))
  (bind _impactpoint (Collision|BreakHitResult _hitresult))
  (if (Game|Player|IsInputKeyDown _returnvalue "LeftMouseButton")
    (SplineMesh|SetEndPosition _splinemesh (+ (SplineMesh|GetStartPosition _splinemesh) _impactpoint) true)
    (Rendering|Debug|DrawDebugPoint _impactpoint 5.0 "(R=1.000000,G=0.000000,B=1.000000,A=1.000000)" 0.0)))

(fn ConstructionScript)