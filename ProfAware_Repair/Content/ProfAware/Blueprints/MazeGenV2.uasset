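; Procedural maze generator that builds a grid of MazeCell floors and cube walls, then carves paths through it.
; Each cell spawns four walls stored in per-direction maps keyed by location, so carving removes both walls between neighbours.
; Tick runs one randomized depth-first backtracking step, using CurrentCell as a stack.
; NewMaze rebuilds after Reset, which destroys every MazeCell, Lamp and StaticMeshActor in the level.
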(event Custom|Generate%20Maze
  (bind _cell_size (Variables|Generation|GetCell%20Size))
  (for _index (range 0 (- (Variables|Generation|GetMaze%20Height) 1))
    (for _index_2 (range 0 (- (Variables|Generation|GetMaze%20Width) 1))
      (Utilities|Array|Add (Variables|Carving|GetAll%20Maze%20Cells) (Math|Vector|MakeVector (Math|Conversions|ToFloat(Integer) (* _index _cell_size)) (Math|Conversions|ToFloat(Integer) (* _index_2 _cell_size)) (.Z (Math|Vector|BreakVector (Variables|Default|GetStart%20Location)))))
      (CallFunction|SpawnFloor (Math|Vector|MakeVector (Math|Conversions|ToFloat(Integer) (* _index _cell_size)) (Math|Conversions|ToFloat(Integer) (* _index_2 _cell_size)) (.Z (Math|Vector|BreakVector (Variables|Default|GetStart%20Location)))))
      (CallFunction|SpawnWalls (Math|Vector|MakeVector (Math|Conversions|ToFloat(Integer) (* _index _cell_size)) (Math|Conversions|ToFloat(Integer) (* _index_2 _cell_size)) (.Z (Math|Vector|BreakVector (Variables|Default|GetStart%20Location))))))))

(event Custom|Spawn%20Floor
  (params (Cell%20Location :type Vector))
  (bind _cell_size (Variables|Generation|GetCell%20Size))
  (bind _returnvalue (/ _cell_size 100))
  (bind _returnvalue_2 (Math|Conversions|ToFloat(Integer) _returnvalue))
  (bind _returnvalue_3 (Game|SpawnActorfromClass "/Game/ProfAware/Blueprints/MazeCell.MazeCell_C" (Math|Transform|MakeTransform Cell%20Location) "Undefined" 0 false 0))
  (Transformation|SetWorldScale3D (Variables|/Game/ProfAware/Blueprints/MazeCell.MazeCell_C|Getbase _returnvalue_3) (Math|Vector|MakeVector _returnvalue_2 _returnvalue_2 0.1)))

(event Custom|Spawn%20Walls
  (params (Cell%20Location :type Vector))
  (bind _maze_wall_height (Variables|Generation|GetMaze%20Wall%20Height))
  (bind _cell_size (Variables|Generation|GetCell%20Size))
  (bind _returnvalue (Math|Conversions|ToFloat(Integer) _cell_size))
  (bind _returnvalue_2 (Math|Conversions|ToFloat(Integer) _maze_wall_height))
  (bind _returnvalue_3 (/ _returnvalue 2.0))
  (bind _returnvalue_4 (/ _returnvalue_2 1e+02))
  (bind _returnvalue_5 (/ _returnvalue_2 2.0))
  (bind _returnvalue_6 (/ _returnvalue 1e+02))
  (bind _returnvalue_7 (Math|Vector|MakeVector _returnvalue_3 0.0 0.0))
  (bind _returnvalue_8 (Math|Vector|MakeVector 0.0 _returnvalue_3 0.0))
  (bind _returnvalue_9 (Math|Vector|MakeVector 0.0 0.0 _returnvalue_5))
  (bind _returnvalue_10 (Math|Vector|MakeVector _returnvalue_6 0.1 _returnvalue_4))
  (bind _returnvalue_11 (Math|Vector|MakeVector 0.1 _returnvalue_6 _returnvalue_4))
  (bind _returnvalue_12 (+ Cell%20Location _returnvalue_9))
  (bind _returnvalue_13 (- _returnvalue_12 _returnvalue_8))
  (bind _returnvalue_14 (- _returnvalue_12 _returnvalue_7))
  (bind _returnvalue_15 (+ _returnvalue_12 _returnvalue_7))
  (bind _returnvalue_16 (+ _returnvalue_12 _returnvalue_8))
  (Utilities|FlowControl|Sequence
    (:then_0
      (bind _returnvalue_17 (Game|SpawnActorfromClass "/Script/Engine.StaticMeshActor" (Math|Transform|MakeTransform _returnvalue_15 "0, 0, 0" _returnvalue_11) "Undefined" 0 0))
      (Utilities|Map|Add (Variables|Walls|GetUp%20Walls) _returnvalue_15 _returnvalue_17)
      (Transformation|SetMobility (Variables|/Script/Engine.StaticMeshActor|GetStaticMeshComponent _returnvalue_17) "Stationary")
      (Components|StaticMesh|SetStaticMesh (Variables|/Script/Engine.StaticMeshActor|GetStaticMeshComponent _returnvalue_17) "/Engine/BasicShapes/Cube.Cube")
      (Rendering|Material|SetMaterial (Variables|/Script/Engine.StaticMeshActor|GetStaticMeshComponent _returnvalue_17) 0 "/Game/PNG/Orange/texture_09_Mat.texture_09_Mat"))
    (:then_1
      (bind _returnvalue_18 (Game|SpawnActorfromClass "/Script/Engine.StaticMeshActor" (Math|Transform|MakeTransform _returnvalue_16 "0, 0, 0" _returnvalue_10) "Undefined" 0 0))
      (Utilities|Map|Add (Variables|Walls|GetRight%20Walls) _returnvalue_16 _returnvalue_18)
      (Transformation|SetMobility (Variables|/Script/Engine.StaticMeshActor|GetStaticMeshComponent _returnvalue_18) "Stationary")
      (Components|StaticMesh|SetStaticMesh (Variables|/Script/Engine.StaticMeshActor|GetStaticMeshComponent _returnvalue_18) "/Engine/BasicShapes/Cube.Cube")
      (Rendering|Material|SetMaterial (Variables|/Script/Engine.StaticMeshActor|GetStaticMeshComponent _returnvalue_18) 0 "/Game/PNG/Orange/texture_09_Mat.texture_09_Mat"))
    (:then_2
      (bind _returnvalue_19 (Game|SpawnActorfromClass "/Script/Engine.StaticMeshActor" (Math|Transform|MakeTransform _returnvalue_14 "0, 0, 0" _returnvalue_11) "Undefined" 0 0))
      (Utilities|Map|Add (Variables|Walls|GetDown%20Walls) _returnvalue_14 _returnvalue_19)
      (Transformation|SetMobility (Variables|/Script/Engine.StaticMeshActor|GetStaticMeshComponent _returnvalue_19) "Stationary")
      (Components|StaticMesh|SetStaticMesh (Variables|/Script/Engine.StaticMeshActor|GetStaticMeshComponent _returnvalue_19) "/Engine/BasicShapes/Cube.Cube")
      (Rendering|Material|SetMaterial (Variables|/Script/Engine.StaticMeshActor|GetStaticMeshComponent _returnvalue_19) 0 "/Game/PNG/Orange/texture_09_Mat.texture_09_Mat"))
    (:then_3
      (bind _returnvalue_20 (Game|SpawnActorfromClass "/Script/Engine.StaticMeshActor" (Math|Transform|MakeTransform _returnvalue_13 "0, 0, 0" _returnvalue_10) "Undefined" 0 0))
      (Utilities|Map|Add (Variables|Walls|GetLeft%20Walls) _returnvalue_13 _returnvalue_20)
      (Transformation|SetMobility (Variables|/Script/Engine.StaticMeshActor|GetStaticMeshComponent _returnvalue_20) "Stationary")
      (Components|StaticMesh|SetStaticMesh (Variables|/Script/Engine.StaticMeshActor|GetStaticMeshComponent _returnvalue_20) "/Engine/BasicShapes/Cube.Cube")
      (Rendering|Material|SetMaterial (Variables|/Script/Engine.StaticMeshActor|GetStaticMeshComponent _returnvalue_20) 0 "/Game/PNG/Orange/texture_09_Mat.texture_09_Mat"))))

(event Custom|Remove%20Up%20Wall
  (bind _current_cell (Variables|Carving|GetCurrent%20Cell))
  (bind _up_walls (Variables|Walls|GetUp%20Walls))
  (bind _maze_wall_height (Variables|Generation|GetMaze%20Wall%20Height))
  (bind _cell_size (Variables|Generation|GetCell%20Size))
  (bind _returnvalue (Math|Conversions|ToFloat(Integer) _maze_wall_height))
  (bind _returnvalue_2 (Math|Conversions|ToFloat(Integer) _cell_size))
  (bind _output (Utilities|Array|Get(acopy) _current_cell))
  (bind _returnvalue_3 (/ _returnvalue 2.0))
  (bind _returnvalue_4 (/ _returnvalue_2 2.0))
  (bind _returnvalue_5 (Math|Vector|MakeVector 0.0 0.0 _returnvalue_3))
  (bind _returnvalue_6 (Math|Vector|MakeVector _returnvalue_4 0.0 0.0))
  (bind _returnvalue_7 (+ _output _returnvalue_5 _returnvalue_6))
  (bind (_value _returnvalue_8) (Utilities|Map|Find _up_walls _returnvalue_7))
  (if _returnvalue_8
    (Actor|DestroyActor _value)))

(event Custom|Remove%20Down%20Wall
  (bind _current_cell (Variables|Carving|GetCurrent%20Cell))
  (bind _maze_wall_height (Variables|Generation|GetMaze%20Wall%20Height))
  (bind _cell_size (Variables|Generation|GetCell%20Size))
  (bind _down_walls (Variables|Walls|GetDown%20Walls))
  (bind _returnvalue (Math|Conversions|ToFloat(Integer) _maze_wall_height))
  (bind _returnvalue_2 (Math|Conversions|ToFloat(Integer) _cell_size))
  (bind _output (Utilities|Array|Get(acopy) _current_cell))
  (bind _returnvalue_3 (/ _returnvalue 2.0))
  (bind _returnvalue_4 (/ _returnvalue_2 2.0))
  (bind _returnvalue_5 (Math|Vector|MakeVector 0.0 0.0 _returnvalue_3))
  (bind _returnvalue_6 (* _returnvalue_4 -1.0))
  (bind _returnvalue_7 (Math|Vector|MakeVector _returnvalue_6 0.0 0.0))
  (bind _returnvalue_8 (+ _output _returnvalue_5 _returnvalue_7))
  (bind (_value _returnvalue_9) (Utilities|Map|Find _down_walls _returnvalue_8))
  (if _returnvalue_9
    (Actor|DestroyActor _value)))

(event Custom|Remove%20Right%20Wall
  (bind _right_walls (Variables|Walls|GetRight%20Walls))
  (bind _current_cell (Variables|Carving|GetCurrent%20Cell))
  (bind _maze_wall_height (Variables|Generation|GetMaze%20Wall%20Height))
  (bind _cell_size (Variables|Generation|GetCell%20Size))
  (bind _returnvalue (Math|Conversions|ToFloat(Integer) _maze_wall_height))
  (bind _returnvalue_2 (Math|Conversions|ToFloat(Integer) _cell_size))
  (bind _output (Utilities|Array|Get(acopy) _current_cell))
  (bind _returnvalue_3 (/ _returnvalue 2.0))
  (bind _returnvalue_4 (/ _returnvalue_2 2.0))
  (bind _returnvalue_5 (Math|Vector|MakeVector 0.0 0.0 _returnvalue_3))
  (bind _returnvalue_6 (Math|Vector|MakeVector 0.0 _returnvalue_4 0.0))
  (bind _returnvalue_7 (+ _output _returnvalue_5 _returnvalue_6))
  (bind (_value _returnvalue_8) (Utilities|Map|Find _right_walls _returnvalue_7))
  (if _returnvalue_8
    (Actor|DestroyActor _value)))

(event Custom|Remove%20Left%20Wall
  (bind _current_cell (Variables|Carving|GetCurrent%20Cell))
  (bind _maze_wall_height (Variables|Generation|GetMaze%20Wall%20Height))
  (bind _cell_size (Variables|Generation|GetCell%20Size))
  (bind _left_walls (Variables|Walls|GetLeft%20Walls))
  (bind _returnvalue (Math|Conversions|ToFloat(Integer) _maze_wall_height))
  (bind _returnvalue_2 (Math|Conversions|ToFloat(Integer) _cell_size))
  (bind _output (Utilities|Array|Get(acopy) _current_cell))
  (bind _returnvalue_3 (/ _returnvalue 2.0))
  (bind _returnvalue_4 (/ _returnvalue_2 2.0))
  (bind _returnvalue_5 (Math|Vector|MakeVector 0.0 0.0 _returnvalue_3))
  (bind _returnvalue_6 (* _returnvalue_4 -1.0))
  (bind _returnvalue_7 (Math|Vector|MakeVector 0.0 _returnvalue_6 0.0))
  (bind _returnvalue_8 (+ _output _returnvalue_5 _returnvalue_7))
  (bind (_value _returnvalue_9) (Utilities|Map|Find _left_walls _returnvalue_8))
  (if _returnvalue_9
    (Actor|DestroyActor _value)))

(event Custom|Carve%20Maze
  (bind _current_cell (Variables|Carving|GetCurrent%20Cell))
  (bind _cell_size (Variables|Generation|GetCell%20Size))
  (bind _returnvalue (Math|Conversions|ToFloat(Integer) _cell_size))
  (bind _output (Utilities|Array|Get(acopy) _current_cell))
  (bind _returnvalue_2 (Math|Vector|MakeVector 0.0 _returnvalue 0.0))
  (bind _returnvalue_3 (Math|Vector|MakeVector _returnvalue 0.0 0.0))
  (bind _returnvalue_4 (- _output _returnvalue_3))
  (bind _returnvalue_5 (- _output _returnvalue_2))
  (bind _returnvalue_6 (+ _output _returnvalue_2))
  (bind _returnvalue_7 (+ _output _returnvalue_3))
  (if (!= (Utilities|Array|Length (Variables|Carving|GetAll%20Visited%20Cells)) (Utilities|Array|Length (Variables|Carving|GetAll%20Maze%20Cells)))
    (if (Math|Boolean|ANDBoolean (Variables|Carving|GetUp%20Flag) (Variables|Carving|GetRight%20Flag) (Variables|Carving|GetDown%20Flag) (Variables|Carving|GetLeft%20Flag))
      (Utilities|Array|RemoveIndex (Variables|Carving|GetCurrent%20Cell))
      (Variables|Carving|SetUp%20Flag false)
      (Variables|Carving|SetRight%20Flag false)
      (Variables|Carving|SetDown%20Flag false)
      (Variables|Carving|SetLeft%20Flag false)
      (else
        (bind _output_get (Variables|Carving|SetRandom%20Int (Math|Random|RandomInteger 4)))
        (switch int _output_get
          (:0
            (if (Math|Boolean|ORBoolean (not (Utilities|Array|ContainsItem (Variables|Carving|GetAll%20Maze%20Cells) _returnvalue_7)) (Utilities|Array|ContainsItem (Variables|Carving|GetAll%20Visited%20Cells) _returnvalue_7) (Variables|Carving|GetUp%20Flag))
              (Variables|Carving|SetUp%20Flag true)
              (else
                (CallFunction|RemoveUpWall)
                (Utilities|Array|Add (Variables|Carving|GetAll%20Visited%20Cells) _returnvalue_7)
                (Utilities|Array|Insert (Variables|Carving|GetCurrent%20Cell) _returnvalue_7)
                (CallFunction|RemoveDownWall))))
          (:1
            (if (Math|Boolean|ORBoolean (not (Utilities|Array|ContainsItem (Variables|Carving|GetAll%20Maze%20Cells) _returnvalue_4)) (Utilities|Array|ContainsItem (Variables|Carving|GetAll%20Visited%20Cells) _returnvalue_4) (Variables|Carving|GetDown%20Flag))
              (Variables|Carving|SetDown%20Flag true)
              (else
                (CallFunction|RemoveDownWall)
                (Utilities|Array|Add (Variables|Carving|GetAll%20Visited%20Cells) _returnvalue_4)
                (Utilities|Array|Insert (Variables|Carving|GetCurrent%20Cell) _returnvalue_4)
                (CallFunction|RemoveUpWall))))
          (:2
            (if (Math|Boolean|ORBoolean (not (Utilities|Array|ContainsItem (Variables|Carving|GetAll%20Maze%20Cells) _returnvalue_6)) (Utilities|Array|ContainsItem (Variables|Carving|GetAll%20Visited%20Cells) _returnvalue_6) (Variables|Carving|GetRight%20Flag))
              (Variables|Carving|SetRight%20Flag true)
              (else
                (CallFunction|RemoveRightWall)
                (Utilities|Array|Add (Variables|Carving|GetAll%20Visited%20Cells) _returnvalue_6)
                (Utilities|Array|Insert (Variables|Carving|GetCurrent%20Cell) _returnvalue_6)
                (CallFunction|RemoveLeftWall))))
          (:3
            (if (Math|Boolean|ORBoolean (not (Utilities|Array|ContainsItem (Variables|Carving|GetAll%20Maze%20Cells) _returnvalue_5)) (Utilities|Array|ContainsItem (Variables|Carving|GetAll%20Visited%20Cells) _returnvalue_5) (Variables|Carving|GetLeft%20Flag))
              (Variables|Carving|SetLeft%20Flag true)
              (else
                (CallFunction|RemoveLeftWall)
                (Utilities|Array|Add (Variables|Carving|GetAll%20Visited%20Cells) _returnvalue_5)
                (Utilities|Array|Insert (Variables|Carving|GetCurrent%20Cell) _returnvalue_5)
                (CallFunction|RemoveRightWall)))))))))

(event Custom|Reset
  (Utilities|FlowControl|Sequence
    (:then_0
      (bind _outactors (Actor|GetAllActorsOfClass "/Game/ProfAware/Blueprints/MazeCell.MazeCell_C"))
      (for _array_element _outactors
        (Actor|DestroyActor _array_element)))
    (:then_1
      (bind _outactors_2 (Actor|GetAllActorsOfClass "/Script/Engine.StaticMeshActor"))
      (for _array_element_2 _outactors_2
        (Actor|DestroyActor _array_element_2)))
    (:then_2
      (bind _outactors_3 (Actor|GetAllActorsOfClass "/Game/ProfAware/Blueprints/Lamp.Lamp_C"))
      (for _array_element_3 _outactors_3
        (Actor|DestroyActor _array_element_3)))
    (:then_3
      (Utilities|Map|Clear (Variables|Walls|GetUp%20Walls))
      (Utilities|Map|Clear (Variables|Walls|GetRight%20Walls))
      (Utilities|Map|Clear (Variables|Walls|GetDown%20Walls))
      (Utilities|Map|Clear (Variables|Walls|GetLeft%20Walls)))
    (:then_5
      (Utilities|Array|Clear (Variables|Carving|GetAll%20Maze%20Cells))
      (Utilities|Array|Clear (Variables|Carving|GetAll%20Visited%20Cells))
      (Utilities|Array|Clear (Variables|Carving|GetCurrent%20Cell)))
    (:then_6
      (Variables|Carving|SetDown%20Flag false)
      (Variables|Carving|SetUp%20Flag false)
      (Variables|Carving|SetRight%20Flag false)
      (Variables|Carving|SetLeft%20Flag false))))

(event Custom|New%20Maze
  (bind _all_maze_cells (Variables|Carving|GetAll%20Maze%20Cells))
  (bind _output (Utilities|Array|Get(acopy) _all_maze_cells))
  (CallFunction|Reset)
  (Utilities|FlowControl|Delay 0.1)
  (CallFunction|GenerateMaze)
  (Utilities|Array|Add (Variables|Carving|GetAll%20Visited%20Cells) _output)
  (Utilities|Array|Insert (Variables|Carving|GetCurrent%20Cell) _output))

(event EventBeginPlay
  (bind _all_maze_cells (Variables|Carving|GetAll%20Maze%20Cells))
  (bind _output (Utilities|Array|Get(acopy) _all_maze_cells))
  (CallFunction|GenerateMaze)
  (Utilities|Array|Add (Variables|Carving|GetAll%20Visited%20Cells) _output)
  (Utilities|Array|Insert (Variables|Carving|GetCurrent%20Cell) _output))

(event EventTick
  (params (DeltaSeconds :type Float%20%28single-precision%29))
  (CallFunction|CarveMaze))

(fn ConstructionScript
  (Variables|Default|SetStart%20Location (Transformation|GetActorLocation)))