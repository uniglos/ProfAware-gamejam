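; Maze generator actor that builds a grid of MazeCell floors with cube wall components, then carves it by randomized depth-first backtracking.
; GenerateMaze runs on BeginPlay, storing cell positions and mapping walls by location.
; Each Tick tries one random neighbor, pushing and tinting it by direction, or pops the stack when all four flags are set.
; Only the "down" branch removes a wall, on the X axis despite moving along Y; other removals are unwired.
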(event Custom|Add%20Side%20Wall
  (params (Location :type Vector))
  (bind (_x _y _z) (Math|Vector|BreakVector Location))
  (bind _cellsize (Variables|MazeAttributes|GetCellSize))
  (bind _returnvalue (/ _cellsize 2.0))
  (bind _returnvalue_2 (- _y _returnvalue))
  (bind _returnvalue_3 (Math|Vector|MakeVector _x _returnvalue_2 _z))
  (bind _returnvalue_4 (AddComponent|AddStaticMeshComponent false))
  (Components|StaticMesh|SetStaticMesh _returnvalue_4 "/Engine/BasicShapes/Cube.Cube")
  (Transformation|SetWorldScale3D _returnvalue_4 (Math|Vector|MakeVector (/ _cellsize 1e+02) 0.1 1.0))
  (Transformation|SetWorldLocation _returnvalue_4 _returnvalue_3 false false)
  (Utilities|Map|Add (Variables|Generation|GetSideWalls) _returnvalue_3 _returnvalue_4))

(event Custom|Add%20Bottom%20Wall
  (params (Location :type Vector))
  (bind (_x _y _z) (Math|Vector|BreakVector Location))
  (bind _cellsize (Variables|MazeAttributes|GetCellSize))
  (bind _returnvalue (/ _cellsize 2.0))
  (bind _returnvalue_2 (- _x _returnvalue))
  (bind _returnvalue_3 (Math|Vector|MakeVector _returnvalue_2 _y _z))
  (bind _returnvalue_4 (AddComponent|AddStaticMeshComponent false))
  (Components|StaticMesh|SetStaticMesh _returnvalue_4 "/Engine/BasicShapes/Cube.Cube")
  (Transformation|SetWorldScale3D _returnvalue_4 (Math|Vector|MakeVector 0.1 (/ _cellsize 1e+02) 1.0))
  (Transformation|SetWorldLocation _returnvalue_4 _returnvalue_3 false false)
  (Utilities|Map|Add (Variables|Generation|GetTopWalls) _returnvalue_3 _returnvalue_4))

(event Custom|Add%20Base
  (params (Location :type Vector))
  (bind (_x _y _z) (Math|Vector|BreakVector Location))
  (bind _cellsize (Variables|MazeAttributes|GetCellSize))
  (bind _returnvalue (/ _cellsize 1e+02))
  (bind _returnvalue_2 (Game|SpawnActorfromClass "/Game/ProfAware/Blueprints/MazeCell.MazeCell_C" (Math|Transform|MakeTransform (Math|Vector|MakeVector _x _y (- _z (/ _cellsize 2.0)))) "Undefined" 0 0))
  (Transformation|SetWorldScale3D (Variables|/Game/ProfAware/Blueprints/MazeCell.MazeCell_C|Getbase _returnvalue_2) (Math|Vector|MakeVector _returnvalue _returnvalue 0.1)))

(event Custom|Add%20Final%20Side%20wall
  (params (Location :type Vector))
  (bind (_x _y _z) (Math|Vector|BreakVector Location))
  (bind _cellsize (Variables|MazeAttributes|GetCellSize))
  (bind _returnvalue (/ _cellsize 2.0))
  (bind _returnvalue_2 (+ _y _returnvalue))
  (bind _returnvalue_3 (Math|Vector|MakeVector _x _returnvalue_2 _z))
  (bind _returnvalue_4 (AddComponent|AddStaticMeshComponent false))
  (Components|StaticMesh|SetStaticMesh _returnvalue_4 "/Engine/BasicShapes/Cube.Cube")
  (Transformation|SetWorldScale3D _returnvalue_4 (Math|Vector|MakeVector (/ _cellsize 1e+02) 0.1 1.0))
  (Transformation|SetWorldLocation _returnvalue_4 _returnvalue_3 false false)
  (Utilities|Map|Add (Variables|Generation|GetSideWalls) _returnvalue_3 _returnvalue_4))

(event Custom|Add%20Final%20Top%20Wall
  (params (Location :type Vector))
  (bind (_x _y _z) (Math|Vector|BreakVector Location))
  (bind _cellsize (Variables|MazeAttributes|GetCellSize))
  (bind _returnvalue (/ _cellsize 2.0))
  (bind _returnvalue_2 (+ _x _returnvalue))
  (bind _returnvalue_3 (Math|Vector|MakeVector _returnvalue_2 _y _z))
  (bind _returnvalue_4 (AddComponent|AddStaticMeshComponent false))
  (Components|StaticMesh|SetStaticMesh _returnvalue_4 "/Engine/BasicShapes/Cube.Cube")
  (Transformation|SetWorldScale3D _returnvalue_4 (Math|Vector|MakeVector 0.1 (/ _cellsize 1e+02) 1.0))
  (Transformation|SetWorldLocation _returnvalue_4 _returnvalue_3 false false)
  (Utilities|Map|Add (Variables|Generation|GetTopWalls) _returnvalue_3 _returnvalue_4))

(event EventBeginPlay
  (bind __mazecells (Variables|Generation|Get%20MazeCells))
  (bind _output (Utilities|Array|Get(acopy) __mazecells))
  (CallFunction|GenerateMaze)
  (Utilities|Array|Add (Variables|Generation|GetVisitedCells) _output)
  (Utilities|Array|Insert (Variables|Generation|GetVisitedCellsStack) _output))

(event EventTick
  (params (DeltaSeconds :type Float%20%28single-precision%29))
  (bind _visitedcellsstack (Variables|Generation|GetVisitedCellsStack))
  (bind _cellsize (Variables|MazeAttributes|GetCellSize))
  (bind _visitedcellsstack_2 (Variables|Generation|GetVisitedCellsStack))
  (bind _visitedcellsstack_3 (Variables|Generation|GetVisitedCellsStack))
  (bind _cellsize_2 (Variables|MazeAttributes|GetCellSize))
  (bind _visitedcellsstack_4 (Variables|Generation|GetVisitedCellsStack))
  (bind _visitedcellsstack_5 (Variables|Generation|GetVisitedCellsStack))
  (bind _cellsize_3 (Variables|MazeAttributes|GetCellSize))
  (bind _visitedcellsstack_6 (Variables|Generation|GetVisitedCellsStack))
  (bind _visitedcellsstack_7 (Variables|Generation|GetVisitedCellsStack))
  (bind _cellsize_4 (Variables|MazeAttributes|GetCellSize))
  (bind _visitedcellsstack_8 (Variables|Generation|GetVisitedCellsStack))
  (bind _topwalls (Variables|Generation|GetTopWalls))
  (bind _visitedcellsstack_9 (Variables|Generation|GetVisitedCellsStack))
  (bind _cellsize_5 (Variables|MazeAttributes|GetCellSize))
  (bind _returnvalue (/ _cellsize_5 2.0))
  (bind _returnvalue_2 (Math|Vector|MakeVector _cellsize 0.0 0.0))
  (bind _returnvalue_3 (Math|Vector|MakeVector _cellsize_2 0.0 0.0))
  (bind _returnvalue_4 (Math|Vector|MakeVector 0.0 _cellsize_3 0.0))
  (bind _returnvalue_5 (Math|Vector|MakeVector 0.0 _cellsize_4 0.0))
  (bind _output (Utilities|Array|Get(acopy) _visitedcellsstack))
  (bind _output_2 (Utilities|Array|Get(acopy) _visitedcellsstack_9 1))
  (bind _output_3 (Utilities|Array|Get(acopy) _visitedcellsstack_3))
  (bind _output_4 (Utilities|Array|Get(acopy) _visitedcellsstack_5))
  (bind _output_5 (Utilities|Array|Get(acopy) _visitedcellsstack_7))
  (bind _returnvalue_6 (Math|Vector|MakeVector _returnvalue 0.0 0.0))
  (bind _returnvalue_7 (- _output _returnvalue_2))
  (bind _returnvalue_8 (- _output_5 _returnvalue_5))
  (bind _returnvalue_9 (+ _output_3 _returnvalue_3))
  (bind _returnvalue_10 (+ _output_4 _returnvalue_4))
  (bind _returnvalue_11 (- _output_2 _returnvalue_6))
  (bind (_value _returnvalue_12) (Utilities|Map|Find _topwalls _returnvalue_11))
  (if (!= (Utilities|Array|Length (Variables|Generation|GetVisitedCells)) (Utilities|Array|Length (Variables|Generation|Get%20MazeCells)))
    (if (Math|Boolean|ANDBoolean (Variables|Default|GetUpFlag) (Variables|Default|GetDownFlag) (Variables|Default|GetLeftFlag) (Variables|Default|GetRightFlag))
      (Utilities|Array|RemoveIndex (Variables|Generation|GetVisitedCellsStack))
      (Variables|Default|SetUpFlag false)
      (Variables|Default|SetLeftFlag false)
      (Variables|Default|SetRightFlag false)
      (Variables|Default|SetDownFlag false)
      (else
        (bind _output_get (Variables|Default|SetRandInt (Math|Random|RandomInteger 4)))
        (switch int _output_get
          (:0
            (Development|PrintString "up" true true "(R=0.000000,G=0.660000,B=1.000000,A=1.000000)" 1e+01)
            (if (Math|Boolean|ORBoolean (not (Utilities|Array|ContainsItem (Variables|Generation|Get%20MazeCells) _returnvalue_9)) (Utilities|Array|ContainsItem (Variables|Generation|GetVisitedCells) _returnvalue_9) (Variables|Default|GetUpFlag))
              (Variables|Default|SetUpFlag true)
              (else
                (Utilities|Array|Add (Variables|Generation|GetVisitedCells) _returnvalue_9)
                (Utilities|Array|Insert _visitedcellsstack_4 _returnvalue_9)
                (bind _outactors (Actor|GetAllActorsOfClass "/Game/ProfAware/Blueprints/MazeCell.MazeCell_C"))
                (bind _asmaze_cell (Utilities|Casting|CastToMazeCell (.ReturnValue (Actor|FindNearestActor (Utilities|Array|Get(acopy) _visitedcellsstack_4) _outactors))))
                (Rendering|Material|SetMaterial (Variables|/Game/ProfAware/Blueprints/MazeCell.MazeCell_C|Getbase _asmaze_cell) 0 "/AnimationSharing/AnimSharingRed.AnimSharingRed"))))
          (:1
            (Development|PrintString "right" true true "(R=0.000000,G=0.660000,B=1.000000,A=1.000000)" 1e+01)
            (if (Math|Boolean|ORBoolean (not (Utilities|Array|ContainsItem (Variables|Generation|Get%20MazeCells) _returnvalue_10)) (Utilities|Array|ContainsItem (Variables|Generation|GetVisitedCells) _returnvalue_10) (Variables|Default|GetRightFlag))
              (Variables|Default|SetRightFlag true)
              (else
                (Utilities|Array|Add (Variables|Generation|GetVisitedCells) _returnvalue_10)
                (Utilities|Array|Insert _visitedcellsstack_6 _returnvalue_10)
                (bind _outactors_2 (Actor|GetAllActorsOfClass "/Game/ProfAware/Blueprints/MazeCell.MazeCell_C"))
                (bind _asmaze_cell_2 (Utilities|Casting|CastToMazeCell (.ReturnValue (Actor|FindNearestActor (Utilities|Array|Get(acopy) _visitedcellsstack_6) _outactors_2))))
                (Rendering|Material|SetMaterial (Variables|/Game/ProfAware/Blueprints/MazeCell.MazeCell_C|Getbase _asmaze_cell_2) 0 "/AnimationSharing/AnimSharingBlue.AnimSharingBlue"))))
          (:2
            (Development|PrintString "down" true true "(R=0.000000,G=0.660000,B=1.000000,A=1.000000)" 1e+01)
            (if (Math|Boolean|ORBoolean (not (Utilities|Array|ContainsItem (Variables|Generation|Get%20MazeCells) _returnvalue_8)) (Utilities|Array|ContainsItem (Variables|Generation|GetVisitedCells) _returnvalue_8) (Variables|Default|GetDownFlag))
              (Variables|Default|SetDownFlag true)
              (else
                (Utilities|Array|Add (Variables|Generation|GetVisitedCells) _returnvalue_8)
                (Utilities|Array|Insert _visitedcellsstack_8 _returnvalue_8)
                (bind _outactors_3 (Actor|GetAllActorsOfClass "/Game/ProfAware/Blueprints/MazeCell.MazeCell_C"))
                (bind _asmaze_cell_3 (Utilities|Casting|CastToMazeCell (.ReturnValue (Actor|FindNearestActor (Utilities|Array|Get(acopy) _visitedcellsstack_8) _outactors_3))))
                (Rendering|Material|SetMaterial (Variables|/Game/ProfAware/Blueprints/MazeCell.MazeCell_C|Getbase _asmaze_cell_3) 0 "/AnimationSharing/AnimSharingGreen.AnimSharingGreen")
                (if _returnvalue_12
                  (Components|DestroyComponent _value)
                  (Utilities|Map|Remove _topwalls _returnvalue_11)))))
          (:3
            (Development|PrintString "left" true true "(R=0.000000,G=0.660000,B=1.000000,A=1.000000)" 1e+01)
            (if (Math|Boolean|ORBoolean (not (Utilities|Array|ContainsItem (Variables|Generation|Get%20MazeCells) _returnvalue_7)) (Utilities|Array|ContainsItem (Variables|Generation|GetVisitedCells) _returnvalue_7) (Variables|Default|GetLeftFlag))
              (Variables|Default|SetLeftFlag true)
              (else
                (Utilities|Array|Add (Variables|Generation|GetVisitedCells) _returnvalue_7)
                (Utilities|Array|Insert _visitedcellsstack_2 _returnvalue_7)
                (bind _outactors_4 (Actor|GetAllActorsOfClass "/Game/ProfAware/Blueprints/MazeCell.MazeCell_C"))
                (bind _asmaze_cell_4 (Utilities|Casting|CastToMazeCell (.ReturnValue (Actor|FindNearestActor (Utilities|Array|Get(acopy) _visitedcellsstack_2) _outactors_4))))
                (Rendering|Material|SetMaterial (Variables|/Game/ProfAware/Blueprints/MazeCell.MazeCell_C|Getbase _asmaze_cell_4) 0 "/DatasmithContent/Materials/AliasMaster.AliasMaster")))))))))

(fn ConstructionScript
  (Variables|Defaults|SetStartLocation (Transformation|GetActorLocation)))

(fn GenerateMaze
  (bind _cellsize (Variables|MazeAttributes|GetCellSize))
  (bind _startlocation (Variables|Defaults|GetStartLocation))
  (for _index (range 0 (- (Variables|MazeAttributes|GetMazeWidth%20%28y%29) 1))
    (for _index_2 (range 0 (- (Variables|MazeAttributes|GetMazeHeight%20%28x%29) 1))
      (CallFunction|AddBase (+ _startlocation (Math|Vector|MakeVector (* (Math|Conversions|ToFloat(Integer) _index_2) _cellsize) (* (Math|Conversions|ToFloat(Integer) _index) _cellsize) (.Z (Math|Vector|BreakVector _startlocation)))))
      (CallFunction|AddSideWall (+ _startlocation (Math|Vector|MakeVector (* (Math|Conversions|ToFloat(Integer) _index_2) _cellsize) (* (Math|Conversions|ToFloat(Integer) _index) _cellsize) (.Z (Math|Vector|BreakVector _startlocation)))))
      (CallFunction|AddBottomWall (+ _startlocation (Math|Vector|MakeVector (* (Math|Conversions|ToFloat(Integer) _index_2) _cellsize) (* (Math|Conversions|ToFloat(Integer) _index) _cellsize) (.Z (Math|Vector|BreakVector _startlocation)))))
      (Utilities|FlowControl|Sequence
        (:then_0
          (if (== _index (- (Variables|MazeAttributes|GetMazeWidth%20%28y%29) 1))
            (CallFunction|AddFinalSideWall (+ _startlocation (Math|Vector|MakeVector (* (Math|Conversions|ToFloat(Integer) _index_2) _cellsize) (* (Math|Conversions|ToFloat(Integer) _index) _cellsize) (.Z (Math|Vector|BreakVector _startlocation)))))))
        (:then_1
          (if (== _index_2 (- (Variables|MazeAttributes|GetMazeHeight%20%28x%29) 1))
            (CallFunction|AddFinalTopWall (+ _startlocation (Math|Vector|MakeVector (* (Math|Conversions|ToFloat(Integer) _index_2) _cellsize) (* (Math|Conversions|ToFloat(Integer) _index) _cellsize) (.Z (Math|Vector|BreakVector _startlocation)))))))
        (:then_2
          (Utilities|Array|Add (Variables|Generation|Get%20MazeCells) (+ _startlocation (Math|Vector|MakeVector (* (Math|Conversions|ToFloat(Integer) _index_2) _cellsize) (* (Math|Conversions|ToFloat(Integer) _index) _cellsize) (.Z (Math|Vector|BreakVector _startlocation))))))))))