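; Player character with walk, yaw look, a Shift sprint and a draining Energy meter.
; Holding Shift raises walk speed and narrows the camera FOV, and a looping timer steadily drains Energy.
; Battery pickup and recharge zone events restore Energy, but only the recharge event caps it.
; Tick just prints "Dead" at zero Energy; vertical look is empty and an upward offset move is unwired.
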(event Custom|Tick%20Health
  (bind _output_get (Variables|Default|SetEnergy (- (Variables|Default|GetEnergy) 0.1)))
  (if (<= _output_get 0.0)
    (Variables|Default|SetEnergy 0.0)))

(event Custom|Battery%20Pickup
  (Variables|Default|SetEnergy (+ (Variables|Default|GetEnergy) 0.3)))

(event Custom|InRechargeZone
  (bind _output_get (Variables|Default|SetEnergy (+ (Variables|Default|GetEnergy) 0.2)))
  (if (>= _output_get 1.0)
    (Variables|Default|SetEnergy 1.0)))

(event EventBeginPlay
  (Utilities|Time|SetTimerbyEvent (delegate Custom|Tick%20Health) 3.0 true))

(event EventTick
  (params (DeltaSeconds :type Float%20%28single-precision%29))
  (if (<= (Variables|Default|GetEnergy) 0.0)
    (Development|PrintString "Dead")))

(event Input|AxisEvents|InputAxisLeft/Right
  (params (AxisValue :type Float%20%28single-precision%29))
  (Pawn|Input|AddMovementInput (Transformation|GetActorRightVector) AxisValue false))

(event Input|AxisEvents|InputAxisUp/Down
  (params (AxisValue :type Float%20%28single-precision%29))
  (Pawn|Input|AddMovementInput (Transformation|GetActorForwardVector) AxisValue false))

(event Input|MouseEvents|MouseX
  (params (AxisValue :type Float%20%28single-precision%29))
  (Pawn|Input|AddControllerYawInput AxisValue))

(event Input|MouseEvents|MouseY
  (params (AxisValue :type Float%20%28single-precision%29)))

(event Input|KeyboardEvents|LeftShift
  (params (Key :type Key%20Structure :default "None"))
  (bind _charactermovement (Variables|Character|GetCharacterMovement))
  (bind _camera (Variables|Default|GetCamera))
  (:Pressed
    (Variables|/Script/Engine.CharacterMovementComponent|SetMaxWalkSpeed _charactermovement 1.2e+03)
    (Camera|SetFieldOfView _camera 7e+01))
  (:Released
    (Variables|/Script/Engine.CharacterMovementComponent|SetMaxWalkSpeed _charactermovement 6e+02)
    (Camera|SetFieldOfView _camera 9e+01)))

(fn ConstructionScript)