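; Repair station actor that the player fixes by holding E, after which it becomes a recharge zone.
; FixZone overlaps flag the player as able to press; Tick polls the key hold, then plays an ActorSequence.
; A DoOnce switches the station on, plays sounds and increments the player's repaired-station count.
; Once on, Tick eases the light radius outward and calls InRechargeZone on nearby players through a one-second Delay.
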(event OnComponentBeginOverlap(FixZone)
  (params (OverlappedComponent :type Primitive%20Component%20Object%20Reference) (OtherActor :type Actor%20Object%20Reference) (OtherComp :type Primitive%20Component%20Object%20Reference) (OtherBodyIndex :type Integer) (bFromSweep :type Boolean) (SweepResult :type Hit%20Result%20Structure%20%28by%20ref%29))
  (bind _returnvalue (Game|GetPlayerCharacter 0))
  (if (== OtherActor _returnvalue)
    (Variables|Default|SetPlayerInZone true)
    (bind _asplayer_character_v2 (Utilities|Casting|CastToPlayerCharacterV2 _returnvalue))
    (Variables|/Game/ProfAware/Blueprints/PlayerCharacterV2.PlayerCharacterV2_C|SetInButtonPushableZone _asplayer_character_v2 true)))

(event OnComponentEndOverlap(FixZone)
  (params (OverlappedComponent :type Primitive%20Component%20Object%20Reference) (OtherActor :type Actor%20Object%20Reference) (OtherComp :type Primitive%20Component%20Object%20Reference) (OtherBodyIndex :type Integer))
  (if (== OtherActor (Game|GetPlayerCharacter 0))
    (Variables|Default|SetPlayerInZone false)
    (bind _asplayer_character_v2 (Utilities|Casting|CastToPlayerCharacterV2 OtherActor))
    (Variables|/Game/ProfAware/Blueprints/PlayerCharacterV2.PlayerCharacterV2_C|SetInButtonPushableZone _asplayer_character_v2 false)))

(event EventBeginPlay)

(event EventTick
  (params (DeltaSeconds :type Float%20%28single-precision%29))
  (bind _pointlight (Variables|Default|GetPointLight))
  (if (Variables|Default|GetOn?)
    (Rendering|Lighting|SetAttenuationRadius _pointlight (Math|Float|Lerp (Variables|/Script/Engine.LocalLightComponent|GetAttenuationRadius _pointlight) 2e+03 0.1))
    (if (<= (Transformation|GetDistanceTo (Game|GetPlayerCharacter 0)) 1e+03)
      (Utilities|FlowControl|Delay 1.0)
      (bind _asplayer_character_v2 (Utilities|Casting|CastToPlayerCharacterV2 (Game|GetPlayerCharacter 0)))
      (Default|InRechargeZone _asplayer_character_v2))
    (elif (Variables|Default|GetPlayerInZone)
      (if (>= (Class|PlayerController|GetInputKeyTimeDown (Game|GetPlayerController 0) "E") 1.0)
        (Sequencer|Player|Play (Variables|/Script/ActorSequence.ActorSequenceComponent|GetSequencePlayer (Variables|Components|GetActorSequence)) :!class /Script/MovieScene.MovieSceneSequencePlayer)
        (Utilities|FlowControl|DoOnce false
          (:Completed
            (Audio|PlaySoundatLocation "/Engine/EditorSounds/GamePreview/EndPlayInEditor.EndPlayInEditor" (Transformation|GetActorLocation) "0, 0, 0" 0.2 0.8 0.0 0 0 0)
            (Variables|Default|SetOn? true)
            (bind _asplayer_character_v2_2 (Utilities|Casting|CastToPlayerCharacterV2 (Game|GetPlayerCharacter 0)))
            (Math|Integer|IncrementInt (Variables|/Game/ProfAware/Blueprints/PlayerCharacterV2.PlayerCharacterV2_C|GetTotalStationsRepaired _asplayer_character_v2_2)
              (:%20%20
                (Audio|Components|Audio|Play (Variables|Default|GetAudio) 0.0)))))))))

(fn ConstructionScript)