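; MazeCell is an actor Blueprint for a maze cell that occasionally places a lamp in the level.
; On BeginPlay it has a 1-in-31 random chance to spawn a Lamp actor at its own location, passing Broken as true.
; The construction script toggles a text render through ShowText, but writes the cell's location into it only on the hidden branch.
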(event EventBeginPlay
  (if (== (Math|Random|RandomInteger 31) 1)
    (Game|SpawnActorfromClass "/Game/ProfAware/Blueprints/Lamp.Lamp_C" (Math|Transform|MakeTransform (Transformation|GetActorLocation)) "Undefined" 0 true 0)))

(event Collision|EventActorBeginOverlap
  (params (OtherActor :type Actor%20Object%20Reference)))

(event EventTick
  (params (DeltaSeconds :type Float%20%28single-precision%29)))

(fn ConstructionScript
  (bind _textrender (Variables|Default|GetTextRender))
  (if (Variables|Default|GetShow%20Text)
    (Rendering|SetVisibility _textrender true false)
    (else
      (Rendering|SetVisibility _textrender false false)
      (Rendering|Components|TextRender|SetText (Variables|Default|GetTextRender) (Utilities|Text|ToText(String) (Transformation|GetActorLocation))))))