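; Spike trap that periodically raises and retracts its spikes and damages the player standing in it.
; A looping timer drives a FlipFlop that sets the target height, plays an attenuated clunk sound and toggles the active state.
; Tick eases all the spike components toward that height with a fixed-alpha lerp.
; While the box overlap flags the player and the trap is active, Tick also calls SpikeDamage on PlayerCharacterV2 every frame.
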(event OnComponentBeginOverlap(Box)
  (params (OverlappedComponent :type Primitive%20Component%20Object%20Reference) (OtherActor :type Actor%20Object%20Reference) (OtherComp :type Primitive%20Component%20Object%20Reference) (OtherBodyIndex :type Integer) (bFromSweep :type Boolean) (SweepResult :type Hit%20Result%20Structure%20%28by%20ref%29))
  (if (== OtherActor (Game|GetPlayerCharacter 0))
    (Variables|Default|SetPlayerInRange true)))

(event OnComponentEndOverlap(Box)
  (params (OverlappedComponent :type Primitive%20Component%20Object%20Reference) (OtherActor :type Actor%20Object%20Reference) (OtherComp :type Primitive%20Component%20Object%20Reference) (OtherBodyIndex :type Integer))
  (if (== OtherActor (Game|GetPlayerCharacter 0))
    (Variables|Default|SetPlayerInRange false)))

(event Custom|ToggleTrap
  (bind _returnvalue (Transformation|GetActorLocation))
  (Utilities|FlowControl|FlipFlop
    (:A
      (Variables|Default|SetPositionOfTrap -195.0)
      (Audio|PlaySoundatLocation "/Game/ProfAware/Sound/lightclunk1.lightclunk1" _returnvalue "0, 0, 0" 1.0 1.0 0.0 "/Game/ProfAware/Sound/SpikeAttenuation.SpikeAttenuation" 0 0)
      (Variables|Default|SetActive false))
    (:B
      (Variables|Default|SetPositionOfTrap 5.0)
      (Audio|PlaySoundatLocation "/Game/ProfAware/Sound/lightclunk2.lightclunk2" _returnvalue "0, 0, 0" 3.0 2.0 0.0 "/Game/ProfAware/Sound/SpikeAttenuation.SpikeAttenuation" 0 0)
      (Variables|Default|SetActive true))))

(event EventBeginPlay
  (Utilities|Time|SetTimerbyEvent (delegate Custom|ToggleTrap) (Variables|Default|GetTrapTime) true))

(event EventTick
  (params (DeltaSeconds :type Float%20%28single-precision%29))
  (if (and (Variables|Default|GetPlayerInRange) (Variables|Default|GetActive))
    (bind _asplayer_character_v2 (Utilities|Casting|CastToPlayerCharacterV2 (Game|GetPlayerCharacter 0)))
    (Default|SpikeDamage _asplayer_character_v2))
  (Utilities|SetSpikePosition (Variables|Default|GetSpike001))
  (Utilities|SetSpikePosition (Variables|Default|GetSpike002))
  (Utilities|SetSpikePosition (Variables|Default|GetSpike003))
  (Utilities|SetSpikePosition (Variables|Default|GetSpike004))
  (Utilities|SetSpikePosition (Variables|Default|GetSpike005))
  (Utilities|SetSpikePosition (Variables|Default|GetSpike006))
  (Utilities|SetSpikePosition (Variables|Default|GetSpike007))
  (Utilities|SetSpikePosition (Variables|Default|GetSpike008))
  (Utilities|SetSpikePosition (Variables|Default|GetSpike009))
  (Utilities|SetSpikePosition (Variables|Default|GetSpike010))
  (Utilities|SetSpikePosition (Variables|Default|GetSpike011))
  (Utilities|SetSpikePosition (Variables|Default|GetSpike012))
  (Utilities|SetSpikePosition (Variables|Default|GetSpike013))
  (Utilities|SetSpikePosition (Variables|Default|GetSpike014))
  (Utilities|SetSpikePosition (Variables|Default|GetSpike0015))
  (Utilities|SetSpikePosition (Variables|Default|GetSpike016))
  (Utilities|SetSpikePosition (Variables|Default|GetSpike017))
  (Utilities|SetSpikePosition (Variables|Default|GetSpike018))
  (Utilities|SetSpikePosition (Variables|Default|GetSpike019))
  (Utilities|SetSpikePosition (Variables|Default|GetSpike020))
  (Utilities|SetSpikePosition (Variables|Default|GetSpike021))
  (Utilities|SetSpikePosition (Variables|Default|GetSpike022))
  (Utilities|SetSpikePosition (Variables|Default|GetSpike023))
  (Utilities|SetSpikePosition (Variables|Default|GetSpike024))
  (Utilities|SetSpikePosition (Variables|Default|GetSpike025))
  (Utilities|SetSpikePosition (Variables|Default|GetSpike026))
  (Utilities|SetSpikePosition (Variables|Default|GetSpike027))
  (Utilities|SetSpikePosition (Variables|Default|GetSpike028))
  (Utilities|SetSpikePosition (Variables|Default|GetSpike029))
  (Utilities|SetSpikePosition (Variables|Default|GetSpike030))
  (Utilities|SetSpikePosition (Variables|Default|GetSpike031))
  (Utilities|SetSpikePosition (Variables|Default|GetSpike032))
  (Utilities|SetSpikePosition (Variables|Default|GetSpike033))
  (Utilities|SetSpikePosition (Variables|Default|GetSpike034))
  (Utilities|SetSpikePosition (Variables|Default|GetSpike035))
  (Utilities|SetSpikePosition (Variables|Default|GetSpike036)))

(fn ConstructionScript)